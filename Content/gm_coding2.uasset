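; Game mode GM_coding2 restores per-level save progress when play begins.
; It checks for a save slot named after the current level, but loads from an empty slot name, or creates a new SG_levelsave if none exists.
; A loaded save runs LoadCollectedCoin and moves the player character's capsule to the stored transform, unless that location is zero.
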(event EventBeginPlay
  (Development|PrintString "Loaded into the GM_coding2")
  (bind _returnvalue (Game|GetCurrentLevelName true))
  (bind _returnvalue_2 (SaveGame|DoesSaveGameExist _returnvalue))
  (if _returnvalue_2
    (bind _returnvalue_3 (SaveGame|LoadGamefromSlot))
    (bind _assg_levelsave (Utilities|Casting|CastToSG_levelsave _returnvalue_3))
    (bind _output_get (Variables|Default|SetLevel%20save _assg_levelsave))
    (Default|LoadCollectedCoin _output_get)
    (if (not (Class|KismetMathLibrary|EqualExactlyVectorVector (.location (Variables|/Game/SG_levelsave.SG_levelsave_C|GetPlayerTransform (Variables|Default|GetLevel%20save))) "0, 0, 0"))
      (Transformation|SetWorldTransform (Variables|/Script/Engine.Character|GetCapsuleComponent (Game|GetPlayerCharacter 0)) (Variables|/Game/SG_levelsave.SG_levelsave_C|GetPlayerTransform (Variables|Default|GetLevel%20save)) false false))
    (else
      (bind _returnvalue_4 (SaveGame|CreateSaveGameObject "/Game/SG_levelsave.SG_levelsave_C"))
      (Variables|Default|SetLevel%20save _returnvalue_4))))

(event EventTick
  (params (DeltaSeconds :type Float%20%28single-precision%29)))

(fn ConstructionScript)