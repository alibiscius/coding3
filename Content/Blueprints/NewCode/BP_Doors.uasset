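; BP_Doors is a door that lowers in a short camera cutscene when OpenDoor is called.
; OpenDoor blends the view to the door, plays a Timeline that slides it down and sets IsOpened, then returns the camera to the passed view target.
; BeginPlay, UpdateDoor and box overlap are empty; the instant-open logic and GameState door-opened notification are disconnected, leaving only the cast.
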(event OnComponentBeginOverlap(Box)
  (params (OverlappedComponent :type Primitive%20Component%20Object%20Reference) (OtherActor :type Actor%20Object%20Reference) (OtherComp :type Primitive%20Component%20Object%20Reference) (OtherBodyIndex :type Integer) (bFromSweep :type Boolean) (SweepResult :type Hit%20Result%20Structure%20%28by%20ref%29))
  ;[1 1 1] Called when collision happens with the door
)

(event Custom|OpenDoor
  (params (NewViewTarget :type Actor%20Object%20Reference))
  (Game|Player|SetViewTargetwithBlend (Game|GetPlayerController 0) self (Variables|Default|GetBlend%20Time) "VTBlend_Cubic" 0.0 true)
  (Utilities|FlowControl|Delay (Variables|Default|GetBlend%20Time))
  (bind _newtrack_0 (Timeline|Timeline Play)
    (:Update
      (Transformation|SetRelativeLocation (Variables|Default|GetDoor) (Math|Vector|Lerp(Vector) "0.000000,0.000000,150.000000" "0.000000,0.000000,-130.000000" _newtrack_0) false false)
      ;[1 1 1] Called when collision happens with the door
      (Variables|Default|SetIsOpened? true)
      ;;[1 1 1] This calls the binded event on the level blueprint by going through the game state
      (bind _asbp_game_state_base (Utilities|Casting|CastToBP_GameStateBase (Game|GetGameState))))
    (:Finished
      (Utilities|FlowControl|Delay 2.0) ; waiting 2 seconds while the door opens
      (Game|Player|SetViewTargetwithBlend (Game|GetPlayerController 0) NewViewTarget (/ (Variables|Default|GetBlend%20Time) 2.0) "VTBlend_Cubic" 0.0 false) ; shift camera back to player
    )))

(event Custom|UpdateDoor
  ;[1 1 1] This event calls from the level blueprint by passing the issue with begin play
)

(event EventBeginPlay
  ;[1 1 1] Event begin plays are called in random order, too many objects to determine which goes first
)

(fn ConstructionScript)