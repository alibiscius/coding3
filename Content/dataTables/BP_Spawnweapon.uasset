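; BP_Spawnweapon is a trigger actor that spawns a random weapon when the third-person character overlaps its Sphere1 component.
; Each overlap picks a random row name from the DT_weapons data table and spawns a BP_weapon at the separate Sphere component's location.
; The row's weapon type and elemental type fill the new weapon's text displays, while the base damage text update is left unconnected.
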(event OnComponentBeginOverlap(Sphere1)
  (params (OverlappedComponent :type Primitive%20Component%20Object%20Reference) (OtherActor :type Actor%20Object%20Reference) (OtherComp :type Primitive%20Component%20Object%20Reference) (OtherBodyIndex :type Integer) (bFromSweep :type Boolean) (SweepResult :type Hit%20Result%20Structure%20%28by%20ref%29))
  (Utilities|Casting|CastToBP_ThirdPersonCharacter OtherActor)
  (CallFunction|SpawnWeapon))

(event Custom|SpawnWeapon
  (bind _outrownames (DataTable|GetDataTableRowNames "/Game/dataTables/DT_weapons.DT_weapons"))
  (bind _returnvalue (Utilities|GetDataTableRow "/Game/dataTables/DT_weapons.DT_weapons" (.OutItem (Utilities|Array|Random _outrownames)))
    (:then
      (bind _returnvalue_2 (Game|SpawnActorfromClass "/Game/dataTables/BP_weapon.BP_weapon_C" (Math|Transform|MakeTransform (Transformation|GetWorldLocation (Variables|Default|GetSphere)) "0, 0, 0" "1.000000,1.000000,1.000000") "Undefined" "MultiplyWithRoot" 0 0))
      (Rendering|Components|TextRender|SetText (Variables|/Game/dataTables/BP_weapon.BP_weapon_C|GetTextweapontype _returnvalue_2) (Utilities|Text|ToText(String) (Utilities|String|EnumtoString (.weapontype _returnvalue))))
      (Rendering|Components|TextRender|SetText (Variables|/Game/dataTables/BP_weapon.BP_weapon_C|GetTextelement _returnvalue_2) (Utilities|Text|ToText(String) (Utilities|String|EnumtoString (.elementaltype _returnvalue)))))))

(event EventBeginPlay)

(event Collision|EventActorBeginOverlap
  (params (OtherActor :type Actor%20Object%20Reference)))

(event EventTick
  (params (DeltaSeconds :type Float%20%28single-precision%29)))

(fn ConstructionScript)