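; BP_weapon is a weapon Blueprint that holds a weapon type, element type and damage range, and displays them as text.
; The randomvalues event adds a small random bonus to the minimum damage, derives the maximum from it with another random offset, then refreshes the text.
; The settext event writes the type and element enum names and the min-max damage range to three text objects.
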(event Custom|set%20text
  (Rendering|Components|TextRender|SetText (Variables|Default|GetTextweapontype) (Utilities|Text|ToText(String) (Utilities|String|EnumtoString (Variables|Default|GetWeapontype))))
  (Rendering|Components|TextRender|SetText (Variables|Default|GetTextelement) (Utilities|Text|ToText(String) (Utilities|String|EnumtoString (Variables|Default|GetElementType))))
  (Rendering|Components|TextRender|SetText (Variables|Default|GetTextDamage) (Utilities|Text|ToText(String) (Utilities|String|Append (Utilities|String|ToString(Integer) (Variables|Default|GetMnDamage)) "-" (Utilities|String|ToString(Integer) (Variables|Default|GetMxDamage))))))

(event Custom|random%20values
  (bind _output_get (Variables|Default|SetMnDamage (+ (Variables|Default|GetMnDamage) (Math|Random|RandomInteger 2))))
  (Variables|Default|SetMxDamage (+ _output_get (Math|Random|RandomIntegerinRange 1 4)))
  (CallFunction|SetText))

(event Collision|EventActorBeginOverlap
  (params (OtherActor :type Actor%20Object%20Reference)))

(event EventTick
  (params (DeltaSeconds :type Float%20%28single-precision%29)))

(fn ConstructionScript)